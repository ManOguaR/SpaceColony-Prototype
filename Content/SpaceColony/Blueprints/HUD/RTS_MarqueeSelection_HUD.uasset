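; RTS HUD that draws a marquee box and selects units inside it.
; Input start clears the previous selection and anchors the box, hold moves its far corner, and release passes the selection to RTS_CameraPawnController_BP.
; While drawing, DrawHUD renders the rectangle and queries GetActorsInSelectionRectangle for RTS_UnitMaster_BP actors every frame.
; Units are added uniquely and pruned when they leave the box, with selection decals updated live.
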(event `self.ReceiveBeginPlay`
  (set `self.ControllerRef` (cast `/Game/SpaceColony/Blueprints/Player/RTS_CameraPawnController_BP` (`GameplayStatics.GetPlayerController` 0) :!pure true)))

(event `/Game/SpaceColony/Blueprints/Library/RTS_MarqueeSelection_IF.OnInputStart`
  (bind (_locationx _locationy) (`PlayerController.GetMousePosition` (`self.ControllerRef`)))
  (if (>= (`KismetArrayLibrary.Array_LastIndex` (`self.SelectedUnits`)) 0)
    (for _array_element (`self.SelectedUnits`)
      (`/Game/SpaceColony/Units/RTS_UnitMaster_BP.SetDeselectedDecal` _array_element))
    (`KismetArrayLibrary.Array_Clear` (`self.SelectedUnits`))
    (`/Game/SpaceColony/Blueprints/Player/RTS_CameraPawnController_BP.ClearSelection` (`self.ControllerRef`)))
  (bind _output_get (set `self.ClickedLocation` (`KismetMathLibrary.MakeVector2D` _locationx _locationy)))
  (set `self.HoldLocation` _output_get)
  (set `self.IsDrawing` true))

(event `/Game/SpaceColony/Blueprints/Library/RTS_MarqueeSelection_IF.OnInputHold`
  (bind (_locationx _locationy) (`PlayerController.GetMousePosition` (`self.ControllerRef`)))
  (set `self.HoldLocation` (`KismetMathLibrary.MakeVector2D` _locationx _locationy))
  (set `self.IsDrawing` true))

(event `/Game/SpaceColony/Blueprints/Library/RTS_MarqueeSelection_IF.OnInputRelease`
  (params (HoldTime :type "Float (single-precision)"))
  (set `self.IsDrawing` false)
  (`/Game/SpaceColony/Blueprints/Player/RTS_CameraPawnController_BP.SetSelectedUnits` (`self.ControllerRef`) (`self.SelectedUnits`)))

(event `self.ReceiveDrawHUD`
  (params (SizeX :type Integer) (SizeY :type Integer))
  (if (`self.IsDrawing`)
    (`|ExecutionSequence`
      (:`then_0`
        (`self.DrawMarquee`)
        (`self.GetSelectedUnitsIfAny`)
        (if (>= (`KismetArrayLibrary.Array_LastIndex` (`self.SelectedUnits`)) 0)
          (for _array_element (`self.SelectedUnits`)
            (`/Game/SpaceColony/Units/RTS_UnitMaster_BP.SetSelectedDecal` _array_element)))))))

(event `DrawMarquee`
  (bind _clickedlocation (`self.ClickedLocation`))
  (bind (_x _y) (`KismetMathLibrary.BreakVector2D` _clickedlocation))
  (bind (_x_2 _y_2) (`KismetMathLibrary.BreakVector2D` (`self.HoldLocation`)))
  (bind (_x_3 _y_3) (`KismetMathLibrary.BreakVector2D` (`self.ClickedLocation`)))
  (bind (_x_4 _y_4) (`KismetMathLibrary.BreakVector2D` (- (`self.HoldLocation`) _clickedlocation)))
  (`self.DrawRect` (struct :`A` 1) _x_3 _y_3)
  (`self.DrawRect` (struct :`A` 1) _x_2 _y_2)
  (`self.DrawRect` (struct :`R` 0.155671 :`G` 1.0 :`B` 0.970151 :`A` 0.5) _x _y _x_4 _y_4))

(fn `GetSelectedUnitsIfAny`
  (locals (SelectedUnitsLocal :type "Array of Actor Object Reference") (CurrentSelectedUnitLocal :type "/Game/SpaceColony/Units/RTS_UnitMaster_BP Object Reference"))
  (bind _returnvalue (`KismetArrayLibrary.Array_LastIndex` (`self.SelectedUnits`)))
  (bind _output_get (set `local.SelectedUnitsLocal` (`self.GetActorsInSelectionRectangle` "/Game/SpaceColony/Units/RTS_UnitMaster_BP.RTS_UnitMaster_BP_C" (`self.ClickedLocation`) (`self.HoldLocation`))))
  (for _array_element _output_get
    (if (`KismetMathLibrary.ClassIsChildOf` (`GameplayStatics.GetObjectClass` _array_element) "/Game/SpaceColony/Units/RTS_UnitMaster_BP.RTS_UnitMaster_BP_C")
      (bind _asrts_unit_master_bp (cast `/Game/SpaceColony/Units/RTS_UnitMaster_BP` _array_element))
      (set `local.CurrentSelectedUnitLocal` _asrts_unit_master_bp)
      (`KismetArrayLibrary.Array_AddUnique` (`self.SelectedUnits`) (`local.CurrentSelectedUnitLocal`))))
  (if (and (> _returnvalue (`KismetArrayLibrary.Array_LastIndex` (`local.SelectedUnitsLocal`))) (>= _returnvalue 0))
    (for _array_element_2 (`self.SelectedUnits`)
      (set `local.CurrentSelectedUnitLocal` _array_element_2)
      (if (not (`KismetArrayLibrary.Array_Contains` (`local.SelectedUnitsLocal`) (`local.CurrentSelectedUnitLocal`)))
        (`KismetArrayLibrary.Array_RemoveItem` (`self.SelectedUnits`) (`local.CurrentSelectedUnitLocal`))
        (`/Game/SpaceColony/Units/RTS_UnitMaster_BP.SetDeselectedDecal` (`local.CurrentSelectedUnitLocal`))))
    (else
      (return))))

(fn `UserConstructionScript`)