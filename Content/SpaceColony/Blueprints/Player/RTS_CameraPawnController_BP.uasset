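; RTS player controller that drives the camera pawn and creates the game clock HUD widget.
; On BeginPlay it caches the camera pawn and game state, then spawns the clock with those references.
; Input handles pawn-relative movement, screen-edge scrolling, a fast-move multiplier, clamped spring-arm zoom and resets.
; Holding Pan opens gates for mouse yaw and clamped pitch rotation while blocking movement; forward movement pins camera height.
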(event `self.ReceiveBeginPlay`
  (`|ExecutionSequence`
    (:`then_0`
      (`self.CastReferences`) ; Must be called first!
    )
    (:`then_1`
      (`self.SpawnWidgets`)
      (`UserWidget.AddToViewport` (`self.HUDGameClockRef`) 0)
      (`self.SetHUDVisibility` "Visible"))))

(event `InputAxis|MoveForward`
  (params (AxisValue :type "Float (single-precision)"))
  ;[1 1 1] Movement Controls
  ;;[1 1 1] Axis Movement
  (if (not (`self.DisableCamMovement`))
    (`self.AxisMovement` AxisValue (stale `InputAxis|MoveRight` AxisValue) :!label _label)))

(event `InputAction|ZoomIn`
  (params (Key :type "Key Structure"))
  (bind _springarm (`/Game/SpaceColony/Blueprints/Player/RTS_CameraPawn_BP.SpringArm` (`self.CameraPawnRef`)))
  ;[1 1 1] Zoom Controls
  ;;[1 1 1] Zoom In
  (:`Pressed`
    (set `SpringArmComponent.TargetArmLength` (`KismetMathLibrary.FClamp` (- (`SpringArmComponent.TargetArmLength` _springarm) (`self.ZoomSpeed`)) (`self.MinZoomLimit`) (`self.MaxZoomLimit`)) _springarm)))

(event `InputAction|FastMoving`
  (params (Key :type "Key Structure"))
  ;[1 1 1] Movement Controls
  ;;[1 1 1] Fast Moving
  (:`Pressed`
    (set `self.CamMoveSpeedMod` 2.0))
  (:`Released`
    (set `self.CamMoveSpeedMod` 1.0)))

(event `InputAxis|MoveRight`
  (params (AxisValue :type "Float (single-precision)"))
  ;[1 1 1] Movement Controls
  ;;[1 1 1] Axis Movement
  (if (not (`self.DisableCamMovement`))
    (goto _label :!via `MovementY`)))

(event `InputAction|ZoomReset`
  (params (Key :type "Key Structure"))
  ;[1 1 1] Zoom Controls
  ;;[1 1 1] Zoom Reset
  (:`Pressed`
    (set `SpringArmComponent.TargetArmLength` (`self.DefaultZoom`) (`/Game/SpaceColony/Blueprints/Player/RTS_CameraPawn_BP.SpringArm` (`self.CameraPawnRef`)))))

(event `InputAxisKey|MouseX`
  (params (AxisValue :type "Float (single-precision)"))
  ;[1 1 1] Movement Controls
  ;;[1 1 1] Edge Scroll Movement
  (if (not (`self.DisableCamMovement`))
    (bind (_deltaspeedx _deltaspeedy) (`self.EdgeScroll` :!label _label_2))
    (`self.K2_AddActorLocalOffset` (`self.CameraPawnRef`) (`KismetMathLibrary.MakeVector` _deltaspeedx _deltaspeedy) true false)))

(event `InputAction|ZoomOut`
  (params (Key :type "Key Structure"))
  (bind _springarm (`/Game/SpaceColony/Blueprints/Player/RTS_CameraPawn_BP.SpringArm` (`self.CameraPawnRef`)))
  ;[1 1 1] Zoom Controls
  ;;[1 1 1] Zoom Out
  (:`Pressed`
    (set `SpringArmComponent.TargetArmLength` (`KismetMathLibrary.FClamp` (+ (`SpringArmComponent.TargetArmLength` _springarm) (`self.ZoomSpeed`)) (`self.MinZoomLimit`) (`self.MaxZoomLimit`)) _springarm)))

(event `InputAxisKey|MouseY`
  (params (AxisValue :type "Float (single-precision)"))
  ;[1 1 1] Movement Controls
  ;;[1 1 1] Edge Scroll Movement
  (if (not (`self.DisableCamMovement`))
    (goto _label_2 :!via `MouseY`)))

(event `InputAxisKey|MouseX`
  (params (AxisValue :type "Float (single-precision)"))
  (bind _camerapawnref (`self.CameraPawnRef`))
  ;[1 1 1] Pan Controls
  ;;[1 1 1] Mouse X Pan
  (`/Engine/EditorBlueprintResources/StandardMacros.Gate` true :!label _label_3
    (:`Exit`
      (`self.K2_SetActorRotation` _camerapawnref (`KismetMathLibrary.MakeRotator` (.roll (`self.K2_GetActorRotation` _camerapawnref)) (.pitch (`self.K2_GetActorRotation` _camerapawnref)) (+ (.yaw (`self.K2_GetActorRotation` _camerapawnref)) (* AxisValue (`self.PanSpeed`)))) false))))

(event `InputAction|Pan`
  (params (Key :type "Key Structure"))
  ;[1 1 1] Pan Controls
  ;;[1 1 1] Mouse X Pan
  (:`Pressed`
    (set `self.DisableCamMovement` true)
    (goto _label_3 :!via `Open`))
  (:`Released`
    (set `self.DisableCamMovement` false)
    (goto _label_3 :!via `Close`)))

(event `InputAction|PanReset`
  (params (Key :type "Key Structure"))
  ;[1 1 1] Pan Controls
  ;;[1 1 1] Pan Reset
  (:`Pressed`
    (`self.K2_SetActorRotation` (`self.CameraPawnRef`) (`KismetMathLibrary.MakeRotator` 0.0) false)))

(event `InputAxisKey|MouseY`
  (params (AxisValue :type "Float (single-precision)"))
  (bind _camerapawnref (`self.CameraPawnRef`))
  ;[1 1 1] Pan Controls
  ;;[1 1 1] Mouse Y Pan
  (`/Engine/EditorBlueprintResources/StandardMacros.Gate` true :!label _label_4
    (:`Exit`
      (`self.K2_SetActorRotation` _camerapawnref (`KismetMathLibrary.MakeRotator` (.roll (`self.K2_GetActorRotation` _camerapawnref)) (`KismetMathLibrary.FClamp` (+ (.pitch (`self.K2_GetActorRotation` _camerapawnref)) (* (`self.PanSpeed`) AxisValue)) -20.0 50.0) (.yaw (`self.K2_GetActorRotation` _camerapawnref))) false))))

(event `InputAction|Pan`
  (params (Key :type "Key Structure"))
  ;[1 1 1] Pan Controls
  ;;[1 1 1] Mouse Y Pan
  (:`Pressed`
    (set `self.DisableCamMovement` true)
    (goto _label_4 :!via `Open`))
  (:`Released`
    (set `self.DisableCamMovement` false)
    (goto _label_4 :!via `Close`)))

(fn `SetHUDVisibility`
  (params (InVisibility :type "ESlateVisibility Enum" :default "Visible"))
  (`Widget.SetVisibility` (`self.HUDGameClockRef`) InVisibility))

(fn `UserConstructionScript`)