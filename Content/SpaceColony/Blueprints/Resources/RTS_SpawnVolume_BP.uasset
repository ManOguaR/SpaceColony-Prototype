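; Spawn volume for the RTS space colony game that places resource actors on the landscape at begin play, on a timer, or both.
; SpawnResource box-traces at random points derived from the volume's bounds and spawns only on Landscape hits.
; Timed spawns skip while the HUD clock is paused or once the requested total reaches its cap.
; RespawnTime follows game speed or user settings each tick, but the looping timer is set only at begin play.
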(event `self.ReceiveBeginPlay`
  (`|ExecutionSequence`
    (:`then_0`
      (`self.CastReferences`))
    (:`then_1`
      (add `/Game/SpaceColony/Blueprints/GameSettings/RTS_GameStateBase_BP.GameSpeedControl` (`self.GameStateRef`) (`|CreateDelegate` :!event `GetGameSpeed`))
      (bind _gamespeed (`/Game/SpaceColony/Blueprints/GameSettings/RTS_GameStateBase_BP.GetGameSpeed` (`self.GameStateRef`)))
      (set `self.GameSpeed` _gamespeed)
      (`self.SetRespawnTimer`))
    (:`then_2`
      (if (`self.IsSpawnOnBeginPlay`)
        (`self.SpawnResource` (`self.ResourceTypeRef`) (`self.CreationAmount`))
        (set `self.TotalNumberSpawned` (+ (`self.CreationAmount`) (`self.TotalNumberSpawned`))))
      (if (and (`self.IsSpawnOnTimer`) (< (`self.TotalNumberSpawned`) (`self.MaxNumberToSpawn`)))
        (`KismetSystemLibrary.K2_SetTimerDelegate` (`|CreateDelegate` :!event `SpawnResourcesOnTimer`) (`self.RespawnTime`) true)))))

(event `GetGameSpeed`
  (params (GameSpeed :type "Float (double-precision)"))
  (set `self.GameSpeed` GameSpeed))

(event `self.ReceiveTick`
  (params (DeltaSeconds :type "Float (single-precision)"))
  (`self.SetRespawnTimer`))

(event `SpawnResourcesOnTimer`
  (if (`/Game/SpaceColony/Blueprints/Widgets/HUD_GameClock_Widget.IsPaused` (`/Game/SpaceColony/Blueprints/Player/RTS_CameraPawnController_BP.HUDGameClockRef` (`self.PlayerControllerRef`)))
    _
    (elif (and (`self.IsSpawnOnTimer`) (< (`self.TotalNumberSpawned`) (`self.MaxNumberToSpawn`)))
      (`self.SpawnResource` (`self.ResourceTypeRef`) (`self.CreationAmount`))
      (set `self.TotalNumberSpawned` (+ (`self.CreationAmount`) (`self.TotalNumberSpawned`))))))

(fn `SetRespawnTimer`
  (returns (RespawnTime :type "Float (double-precision)"))
  (switch `/Game/SpaceColony/Blueprints/Enums/RespawnTimerEnum` (`self.TimeSetting`)
    (:`NewEnumerator1`
      (set `self.RespawnTime` 0.0))
    (:`NewEnumerator2`
      (set `self.RespawnTime` (`self.GameSpeed`)))
    (:`NewEnumerator3`
      (set `self.RespawnTime` (`self.UserRespawnTimer`)))
    (:`NewEnumerator4`
      (set `self.RespawnTime` (* (`self.GameSpeed`) (`self.UserRespawnTimer`)))))
  (return 0.0))

(fn `SpawnResource`
  (params (ResourceType :type "/Game/SpaceColony/Blueprints/Resources/RTS_ResourceMaster_BP Class Reference") (ResourceAmount :type Integer))
  (locals (ResourceTypeRefLocal :type "/Game/SpaceColony/Blueprints/Resources/RTS_ResourceMaster_BP Class Reference") (ResorceAmountLocal :type Integer))
  (bind (_origin _boxextent) (`self.GetActorBounds` false))
  (bind _x (.x _boxextent))
  (bind _y (.y _boxextent))
  (bind _returnvalue (+ _origin (`KismetMathLibrary.MakeVector` (`KismetMathLibrary.RandomFloatInRange` (- _x (* _x 2.0)) _x) (`KismetMathLibrary.RandomFloatInRange` (- _y (* _y 2.0)) _y) (.z _origin))))
  (set `local.ResourceTypeRefLocal` ResourceType)
  (set `local.ResorceAmountLocal` ResourceAmount)
  (for _ (range 1 (+ (`local.ResorceAmountLocal`) 1))
    (bind _outhit (`KismetSystemLibrary.BoxTraceSingle` (+ _returnvalue (0.0 0.0 200.0)) (0.0 0.0 0.0) (- _returnvalue (0.0 0.0 200.0)) (struct) "TraceTypeQuery1"))
    (bind (_bblockinghit _binitialoverlap _time _distance _location _impactpoint _normal _impactnormal _physmat _hitactor) (`GameplayStatics.BreakHitResult` _outhit))
    (if (== (`GameplayStatics.GetObjectClass` _hitactor) "/Script/Landscape.Landscape")
      (`|SpawnActorFromClass` (`local.ResourceTypeRefLocal`) (`KismetMathLibrary.Conv_VectorToTransform` _location) "Undefined" "OverrideRootScale" null null))))

(fn `UserConstructionScript`)